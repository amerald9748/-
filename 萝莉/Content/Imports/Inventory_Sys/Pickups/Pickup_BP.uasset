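; Pickup actor that gives an item class and amount to the player's inventory on overlap and bobs in place.
; Overlap with a TPDefaultChar calls AddItem on its inventory reference.
; A successful add keeps any leftover as the new amount or destroys the actor when none remains, while a failed add prints a message.
; Tick plays the Bob timeline, whose track drives a local offset on each update.
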(event `self.ReceiveActorBeginOverlap`
  (params (OtherActor :type "Actor Object Reference"))
  (bind _astpdefault_char (cast `/Game/Imports/TPDefaultChar` OtherActor))
  (bind _inventoryref (`/Game/Imports/TPDefaultChar.InventoryRef` _astpdefault_char))
  (`/Engine/EditorBlueprintResources/StandardMacros.IsValid` _inventoryref
    (:`Is Valid`
      (bind (_success _rest) (`/Game/Imports/Inventory_Sys/Inventory_BP.AddItem` _inventoryref (`self.ItemToAdd`) (`self.AmountToAdd`)))
      (if _success
        (if (> _rest 0)
          (set `self.AmountToAdd` _rest)
          (else
            (`self.K2_DestroyActor`)))
        (else
          (`KismetSystemLibrary.PrintString` "failed"))))))

(event `self.ReceiveTick`
  (params (DeltaSeconds :type "Float (single-precision)"))
  (bind (_direction _newtrack_0) (`Timeline|Bob`)
    (:`Update`
      (`self.K2_AddActorLocalOffset` _newtrack_0))))

(fn `UserConstructionScript`)
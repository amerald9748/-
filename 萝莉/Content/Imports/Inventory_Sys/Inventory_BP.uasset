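; Slot-based inventory actor that stores item classes with amounts and creates the main inventory widget on BeginPlay.
; AddItem fills free stacks, then empty slots, recursing on overflow and returning any rest.
; Functions remove, swap, merge and split stacks, refreshing affected slot widgets by index.
; Item info comes from class defaults, so an item actor is spawned only on use to run EventOnUse.
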(event `self.ReceiveBeginPlay`
  (`KismetArrayLibrary.Array_Resize` (`self.Slots`) (`self.AmountSlot`))
  (bind _returnvalue (`|CreateWidget` "/Game/Imports/HUD/MainWidget.MainWidget_C" null self (`self.SlotsPerRow`)))
  (bind _output_get (set `self.MainWidget` _returnvalue))
  (set `self.InventoryWidget` (`/Game/Imports/HUD/MainWidget.Inventory_Widget` _output_get))
  (`UserWidget.AddToViewport` (`self.MainWidget`) 0))

(event `UpdateSlotAtIndex`
  (params (Index :type Integer))
  (`/Game/Imports/HUD/InventorySlot.UpdateSlot` (`KismetArrayLibrary.Array_Get` (`/Game/Imports/HUD/Inventory.SlotsWidget` (`self.InventoryWidget`)) Index)))

(event `UseItemAtIndex`
  (params (Index :type Integer))
  (bind _item_itemclass (break `/Game/Imports/Inventory_Sys/SlotStruct` (`KismetArrayLibrary.Array_Get` (`self.Slots`) Index)))
  (if (`KismetSystemLibrary.IsValidClass` _item_itemclass)
    (bind _returnvalue (`|SpawnActorFromClass` _item_itemclass (`KismetMathLibrary.MakeTransform` (0.0 0.0 0.0)) "AlwaysSpawn" "OverrideRootScale" null self Index))
    (`/Game/Imports/Inventory_Sys/Pickups/MasterItemClass_BP.EventOnUse` _returnvalue)))

(fn `AddItem`
  (params (ItemClass :type "/Game/Imports/Inventory_Sys/Pickups/MasterItemClass_BP Class Reference") (Amount :type Integer))
  (returns (Success :type Boolean) (Rest :type Integer))
  (locals (LocalClass :type "/Game/Imports/Inventory_Sys/Pickups/MasterItemClass_BP Class Reference") (LocalAmount :type Integer) (FoundIndex :type Integer))
  (bind _localamount (`local.LocalAmount`))
  (bind _foundindex (`local.FoundIndex`))
  (bind _maxstacksize (`self.MaxStackSize`))
  (bind _foundindex_2 (`local.FoundIndex`))
  (bind _foundindex_3 (`local.FoundIndex`))
  (bind _localclass (`local.LocalClass`))
  (bind (_item_itemclass _item_amount) (break `/Game/Imports/Inventory_Sys/SlotStruct` (`KismetArrayLibrary.Array_Get` (`self.Slots`) (`local.FoundIndex`))))
  (bind _returnvalue (+ _item_amount (`local.LocalAmount`)))
  (set `local.LocalAmount` Amount)
  (set `local.LocalClass` ItemClass)
  (if (`.CanBeStacked?_20_3B42217C4279F98B858FC993C01256C1` (break `/Game/Imports/Inventory_Sys/InventoryStruct` (`.ItemInfo` (defaults `/Game/Imports/Inventory_Sys/Inventory_BP` ItemClass))))
    (bind (_success _index) (`self.SearchFreeStack` (`local.LocalClass`)))
    (if _success
      (set `local.FoundIndex` _index)
      (if (> _returnvalue _maxstacksize)
        (bind _output_get (set `local.LocalAmount` (- _returnvalue _maxstacksize)))
        (`KismetArrayLibrary.Array_Set` (`self.Slots`) _foundindex_2 (make `/Game/Imports/Inventory_Sys/SlotStruct` _localclass _maxstacksize))
        (`self.UpdateSlotAtIndex` _foundindex_2)
        (bind (_success_2 _rest) (`self.AddItem` _localclass _output_get))
        (return true _rest)
        (else
          (`KismetArrayLibrary.Array_Set` (`self.Slots`) _foundindex_3 (make `/Game/Imports/Inventory_Sys/SlotStruct` (`local.LocalClass`) _returnvalue))
          (`self.UpdateSlotAtIndex` _foundindex_3)
          (return true 0)))
      (else
        (bind (_success_3 _index_2) (`self.SearchEmptySlot`))
        (if _success_3
          (bind _output_get_2 (set `local.FoundIndex` _index_2))
          (if (> _localamount (`self.MaxStackSize`))
            (`KismetArrayLibrary.Array_Set` (`self.Slots`) _output_get_2 (make `/Game/Imports/Inventory_Sys/SlotStruct` (`local.LocalClass`) (`self.MaxStackSize`)))
            (`self.UpdateSlotAtIndex` (`local.FoundIndex`))
            (bind (_success_4 _rest_2) (`self.AddItem` (`local.LocalClass`) (- (`local.LocalAmount`) (`self.MaxStackSize`))))
            (return _success_4 _rest_2)
            (else
              (`KismetArrayLibrary.Array_Set` (`self.Slots`) _foundindex (make `/Game/Imports/Inventory_Sys/SlotStruct` (`local.LocalClass`) (`local.LocalAmount`)))
              (`self.UpdateSlotAtIndex` _foundindex)
              (return true 0)))
          (else
            (`KismetSystemLibrary.PrintString` "No Empty Slot or Free Stacks found")
            (return false _localamount)))))
    (else
      (bind (_success_5 _index_3) (`self.SearchEmptySlot`))
      (if _success_5
        (bind _output_get_3 (set `local.FoundIndex` _index_3))
        (`KismetArrayLibrary.Array_Set` (`self.Slots`) _output_get_3 (make `/Game/Imports/Inventory_Sys/SlotStruct` (`local.LocalClass`) 1))
        (`self.UpdateSlotAtIndex` (`local.FoundIndex`))
        (if (> (`local.LocalAmount`) 1)
          (bind (_success_6 _rest_3) (`self.AddItem` (`local.LocalClass`) (- (`local.LocalAmount`) 1)))
          (return _success_6 _rest_3)
          (else
            (return true 0)))
        (else
          (`KismetSystemLibrary.PrintString` "No Empty Slots Found")
          (return false (`local.LocalAmount`)))))))

(fn `AddToIndex`
  (params (FromIndex :type Integer) (ToIndex :type Integer))
  (returns (`Success?` :type Boolean))
  (locals (LocalFrom :type Integer) (LocalTo :type Integer) (LocalClass :type "/Game/Imports/Inventory_Sys/Pickups/MasterItemClass_BP Class Reference"))
  (bind _slots (`self.Slots`))
  (bind (_item_itemclass _item_amount) (break `/Game/Imports/Inventory_Sys/SlotStruct` (`KismetArrayLibrary.Array_Get` (`self.Slots`) (`local.LocalTo`))))
  (bind _item_itemclass_2 (break `/Game/Imports/Inventory_Sys/SlotStruct` (`KismetArrayLibrary.Array_Get` (`self.Slots`) (`local.LocalFrom`))))
  (set `local.LocalFrom` FromIndex)
  (set `local.LocalTo` ToIndex)
  (if (and (== _item_itemclass_2 _item_itemclass) (< _item_amount (`self.MaxStackSize`)) (`.CanBeStacked?_20_3B42217C4279F98B858FC993C01256C1` (break `/Game/Imports/Inventory_Sys/InventoryStruct` (`.ItemInfo` (`self.GetItemInfoAtIndex` (`local.LocalFrom`))))))
    (set `local.LocalClass` _item_itemclass_2)
    (if (>= (- (`self.MaxStackSize`) (`self.GetAmountAtIndex` (`local.LocalTo`))) (`self.GetAmountAtIndex` (`local.LocalFrom`)))
      (`KismetArrayLibrary.Array_Set` _slots (`local.LocalTo`) (make `/Game/Imports/Inventory_Sys/SlotStruct` (`local.LocalClass`) (+ (`self.GetAmountAtIndex` (`local.LocalFrom`)) (`self.GetAmountAtIndex` (`local.LocalTo`)))))
      (`KismetArrayLibrary.Array_Set` _slots (`local.LocalFrom`) (make `/Game/Imports/Inventory_Sys/SlotStruct` null))
      (else
        (`KismetArrayLibrary.Array_Set` _slots (`local.LocalFrom`) (make `/Game/Imports/Inventory_Sys/SlotStruct` (`local.LocalClass`) (- (`self.GetAmountAtIndex` (`local.LocalFrom`)) (- (`self.MaxStackSize`) (`self.GetAmountAtIndex` (`local.LocalTo`))))))
        (`KismetArrayLibrary.Array_Set` (`self.Slots`) (`local.LocalTo`) (make `/Game/Imports/Inventory_Sys/SlotStruct` (`local.LocalClass`) (`self.MaxStackSize`)))))
    (`self.UpdateSlotAtIndex` (`local.LocalFrom`))
    (`self.UpdateSlotAtIndex` (`local.LocalTo`))
    (return true)
    (else
      (return false))))

(fn `GetAmountAtIndex`
  (params (Index :type Integer))
  (returns (Amount :type Integer))
  (bind (_item_itemclass _item_amount) (break `/Game/Imports/Inventory_Sys/SlotStruct` (`KismetArrayLibrary.Array_Get` (`self.Slots`) Index)))
  (return _item_amount))

(fn `GetItemInfoAtIndex`
  (params (Index :type Integer))
  (returns (`EmptySlot?` :type Boolean) (ItemInfo :type "/Game/Imports/Inventory_Sys/InventoryStruct Structure") (Amount :type Integer))
  (bind (_item_itemclass _item_amount) (break `/Game/Imports/Inventory_Sys/SlotStruct` (`KismetArrayLibrary.Array_Get` (`self.Slots`) Index)))
  (if (`KismetSystemLibrary.IsValidClass` _item_itemclass)
    (return false (`.ItemInfo` (defaults `/Game/Imports/Inventory_Sys/Inventory_BP` _item_itemclass)) _item_amount)
    (else
      (return true (struct) 0))))

(fn `HideInv`
  (bind _inventorywidget (`self.InventoryWidget`))
  (`Widget.SetVisibility` _inventorywidget "Hidden")
  (set `self.IsVisible?` false)
  (`Widget.SetIsEnabled` _inventorywidget false)
  (`Widget.SetVisibility` (`self.MainWidget`) "Hidden")
  (`Widget.SetIsEnabled` (`/Game/Imports/HUD/Inventory.SlotPanel` (`self.InventoryWidget`)) true)
  (return))

(fn `IsSlotEmpty?`
  (params (Index :type Integer))
  (returns (`Empty?` :type Boolean))
  (bind _item_itemclass (break `/Game/Imports/Inventory_Sys/SlotStruct` (`KismetArrayLibrary.Array_Get` (`self.Slots`) Index)))
  (return (not (`KismetSystemLibrary.IsValidClass` _item_itemclass))))

(fn `RemoveItemAtIndex`
  (params (Index :type Integer) (Amount :type Integer))
  (returns (`Success?` :type Boolean))
  (locals (LocalIndex :type Integer) (LocalAmount :type Integer))
  (bind _slots (`self.Slots`))
  (bind _localindex (`local.LocalIndex`))
  (bind (_item_itemclass _item_amount) (break `/Game/Imports/Inventory_Sys/SlotStruct` (`KismetArrayLibrary.Array_Get` _slots (`local.LocalIndex`))))
  (set `local.LocalIndex` Index)
  (set `local.LocalAmount` Amount)
  (if (and (not (`self.IsSlotEmpty?` (`local.LocalIndex`))) (> (`local.LocalAmount`) 0))
    (if (>= (`local.LocalAmount`) (`self.GetAmountAtIndex` (`local.LocalIndex`)))
      (`KismetArrayLibrary.Array_Set` _slots _localindex (make `/Game/Imports/Inventory_Sys/SlotStruct` null))
      (`self.UpdateSlotAtIndex` _localindex)
      (return true)
      (else
        (`KismetArrayLibrary.Array_Set` _slots _localindex (make `/Game/Imports/Inventory_Sys/SlotStruct` _item_itemclass (- _item_amount (`local.LocalAmount`))))
        (`self.UpdateSlotAtIndex` (`local.LocalIndex`))
        (return true)))
    (else
      (return false))))

(fn `SearchEmptySlot`
  (returns (Success :type Boolean) (Index :type Integer))
  (locals (LocalBool :type Boolean) (LocalIndex :type Integer))
  (for (_array_element _array_index) (`self.Slots`)
    (if (not (`KismetSystemLibrary.IsValidClass` (break `/Game/Imports/Inventory_Sys/SlotStruct` _array_element)))
      (set `local.LocalBool` true)
      (set `local.LocalIndex` _array_index)
      (break)))
  (return (`local.LocalBool`) (`local.LocalIndex`)))

(fn `SearchFreeStack`
  (params (ItemClass :type "/Game/Imports/Inventory_Sys/Pickups/MasterItemClass_BP Class Reference"))
  (returns (Success :type Boolean) (Index :type Integer))
  (locals (LocalIndex :type Integer) (LocalBool :type Boolean))
  (for (_array_element _array_index) (`self.Slots`)
    (if (`KismetSystemLibrary.IsValidClass` (break `/Game/Imports/Inventory_Sys/SlotStruct` _array_element))
      (if (and (== (break `/Game/Imports/Inventory_Sys/SlotStruct` _array_element) ItemClass) (< (`.Amount_10_542ABD404F615FBB4750D6BB696CE7D0` (break `/Game/Imports/Inventory_Sys/SlotStruct` _array_element)) (`self.MaxStackSize`)))
        (set `local.LocalBool` true)
        (set `local.LocalIndex` _array_index)
        (break))))
  (return (`local.LocalBool`) (`local.LocalIndex`)))

(fn `ShowInv`
  (bind _inventorywidget (`self.InventoryWidget`))
  (`Widget.SetVisibility` _inventorywidget "Visible")
  (set `self.IsVisible?` true)
  (`Widget.SetIsEnabled` _inventorywidget true)
  (return))

(fn `SplitStacks`
  (params (StackIndex :type Integer) (Amount :type Integer))
  (returns (`Success?` :type Boolean))
  (locals (LocalStackIndex :type Integer) (LocalAmount :type Integer) (LocalFoundIndex :type Integer :default 0))
  (bind _localstackindex (`local.LocalStackIndex`))
  (bind (_item_itemclass _item_amount) (break `/Game/Imports/Inventory_Sys/SlotStruct` (`KismetArrayLibrary.Array_Get` (`self.Slots`) (`local.LocalStackIndex`))))
  (bind (_emptyslot_ _iteminfo _amount) (`self.GetItemInfoAtIndex` _localstackindex))
  (set `local.LocalStackIndex` StackIndex)
  (set `local.LocalAmount` Amount)
  (if (`self.IsSlotEmpty?` _localstackindex)
    (return false)
    (elif (and (`.CanBeStacked?_20_3B42217C4279F98B858FC993C01256C1` (break `/Game/Imports/Inventory_Sys/InventoryStruct` _iteminfo)) (> _amount (`local.LocalAmount`)))
      (bind (_success _index) (`self.SearchEmptySlot`))
      (if _success
        (set `local.LocalFoundIndex` _index)
        (`KismetArrayLibrary.Array_Set` (`self.Slots`) (`local.LocalStackIndex`) (make `/Game/Imports/Inventory_Sys/SlotStruct` _item_itemclass (- _item_amount (`local.LocalAmount`))))
        (`KismetArrayLibrary.Array_Set` (`self.Slots`) (`local.LocalFoundIndex`) (make `/Game/Imports/Inventory_Sys/SlotStruct` _item_itemclass (`local.LocalAmount`)))
        (`self.UpdateSlotAtIndex` (`local.LocalStackIndex`))
        (`self.UpdateSlotAtIndex` (`local.LocalFoundIndex`))
        (return true)
        (else
          (return false)))
      (else
        (return false)))))

(fn `SplitStackToIndex`
  (params (FromIndex :type Integer) (ToIndex :type Integer) (Amount :type Integer))
  (returns (`Success?` :type Boolean))
  (locals (LocalFrom :type Integer) (LocalTo :type Integer) (LocalAmount :type Integer) (LocalClass :type "/Game/Imports/Inventory_Sys/Pickups/MasterItemClass_BP Class Reference"))
  (bind _slots (`self.Slots`))
  (bind (_item_itemclass _item_amount) (break `/Game/Imports/Inventory_Sys/SlotStruct` (`KismetArrayLibrary.Array_Get` _slots (`local.LocalFrom`))))
  (bind _output_get (set `local.LocalFrom` FromIndex))
  (bind _output_get_2 (set `local.LocalTo` ToIndex))
  (set `local.LocalAmount` Amount)
  (bind (_emptyslot_ _iteminfo _amount) (`self.GetItemInfoAtIndex` _output_get))
  (if (and (`self.IsSlotEmpty?` _output_get_2) (not (`self.IsSlotEmpty?` _output_get)) (`.CanBeStacked?_20_3B42217C4279F98B858FC993C01256C1` (break `/Game/Imports/Inventory_Sys/InventoryStruct` _iteminfo)) (> _amount 1) (> _amount (`local.LocalAmount`)))
    (bind _output_get_3 (set `local.LocalClass` _item_itemclass))
    (`KismetArrayLibrary.Array_Set` _slots (`local.LocalFrom`) (make `/Game/Imports/Inventory_Sys/SlotStruct` _output_get_3 (- _item_amount (`local.LocalAmount`))))
    (`KismetArrayLibrary.Array_Set` (`self.Slots`) (`local.LocalTo`) (make `/Game/Imports/Inventory_Sys/SlotStruct` (`local.LocalClass`) (`local.LocalAmount`)))
    (`self.UpdateSlotAtIndex` (`local.LocalFrom`))
    (`self.UpdateSlotAtIndex` (`local.LocalTo`))
    (return true)
    (else
      (return false))))

(fn `SwapSlots`
  (params (Index1 :type Integer) (Index2 :type Integer))
  (returns (`Success?` :type Boolean))
  (locals (LocalIndex1 :type Integer) (LocalIndex2 :type Integer) (LocalSlot2 :type "/Game/Imports/Inventory_Sys/SlotStruct Structure"))
  (bind _localindex2 (`local.LocalIndex2`))
  (bind _localindex1 (`local.LocalIndex1`))
  (bind _slots (`self.Slots`))
  (bind _slots_2 (`self.Slots`))
  (set `local.LocalIndex1` Index1)
  (set `local.LocalIndex2` Index2)
  (if (or (> (`local.LocalIndex1`) (`KismetArrayLibrary.Array_LastIndex` _slots)) (> (`local.LocalIndex2`) (`KismetArrayLibrary.Array_LastIndex` _slots)))
    (return false)
    (else
      (bind _output_get (set `local.LocalSlot2` (`KismetArrayLibrary.Array_Get` (`self.Slots`) _localindex2)))
      (`KismetArrayLibrary.Array_Set` _slots_2 _localindex2 (`KismetArrayLibrary.Array_Get` (`self.Slots`) _localindex1))
      (`KismetArrayLibrary.Array_Set` _slots_2 _localindex1 _output_get)
      (`self.UpdateSlotAtIndex` (`local.LocalIndex1`))
      (`self.UpdateSlotAtIndex` (`local.LocalIndex2`))
      (return true))))

(fn `UserConstructionScript`)